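; Item use action for a door stone key that unlocks a matching door in front of the player.
; UseEvent overrides the parent and sphere-traces forward from the player pawn for WorldDynamic objects, casting the hit to BP_Master_Door.
; If the door's KeyID matches the inventory item's, it unlocks the door and removes the item when flagged DiscardWhenUsed.
; The action actor destroys itself after hitting a door, whether or not the key matched.
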(event `self.ReceiveBeginPlay`
  ;[0 0.7682 1] Call startup sequence from parent
  (`parent.ReceiveBeginPlay`))

(event `self.UseEvent`
  (bind _returnvalue (`GameplayStatics.GetPlayerPawn` 0))
  (bind _returnvalue_2 (`self.K2_GetActorLocation` _returnvalue))
  (bind ((`KeyID_45_913559F04778E4BD017181B2929637FA` _keyid) (`DiscardWhenUsed?_28_8EB76B144DE06174AED7C29762E05C3D` _discardwhenused_)) (break `/Game/StoryAdvTemplate/Blueprints/Data/Structures/BP_InventoryItem` (`|GetArrayItem` (`/Game/StoryAdvTemplate/Blueprints/BP_GameController.Inventory` (`self.GameController`)) (`self.ItemInventoryIndex`))))
  ;[0 0.7682 1] Use Event: Search for a door in front of character, then try to open it
  (bind (_outhit _returnvalue_3) (`KismetSystemLibrary.SphereTraceSingleForObjects` _returnvalue_2 (+ _returnvalue_2 (* (`self.GetActorForwardVector` _returnvalue) 200.0)) 20.0 (`|MakeArray` "ObjectTypeQuery2" :!type "EObjectTypeQuery Enum") false (`|MakeArray` (`GameplayStatics.GetPlayerPawn` 0) :!type "Actor Object Reference")))
  (if _returnvalue_3
    (bind _asbp_master_door (cast `/Game/StoryAdvTemplate/Blueprints/MasterBlueprints/Doors/BP_Master_Door` (`.HitActor` (`GameplayStatics.BreakHitResult` _outhit))))
    (if (== (`/Game/StoryAdvTemplate/Blueprints/MasterBlueprints/Doors/BP_Master_Door.KeyID` _asbp_master_door) _keyid)
      (`/Game/StoryAdvTemplate/Blueprints/MasterBlueprints/Doors/BP_Master_Door.UnlockDoor` _asbp_master_door)
      (if _discardwhenused_
        (`KismetArrayLibrary.Array_Remove` (`/Game/StoryAdvTemplate/Blueprints/BP_GameController.Inventory` (`self.GameController`)) (`self.ItemInventoryIndex`))))
    (`self.K2_DestroyActor`)))

(fn `UserConstructionScript`
  (`parent.UserConstructionScript`))